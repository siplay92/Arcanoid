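; Block actor that the ball breaks by hitting it, losing one life per hit.
; The Hit event casts the other actor to Ball, decrements Lives, then either swaps the Cube's material through a Select indexed by remaining lives or destroys the block itself at zero.
; Each hit logs the cube's name and remaining lives without printing to screen.
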(event Custom|CustomEvent)

(event Collision|EventActorBeginOverlap
  (params (OtherActor :type Actor%20Object%20Reference)))

(event Collision|EventHit
  (params (MyComp :type Primitive%20Component%20Object%20Reference) (Other :type Actor%20Object%20Reference) (OtherComp :type Primitive%20Component%20Object%20Reference) (bSelfMoved :type Boolean) (HitLocation :type Vector :default "0, 0, 0") (HitNormal :type Vector :default "0, 0, 0") (NormalImpulse :type Vector :default "0, 0, 0") (Hit :type Hit%20Result%20Structure%20%28by%20ref%29))
  ;[1 1 1] когда проиходит hit, преобразуем и проверяем шарик ли это и уменьшаем количество жизней
  (Utilities|Casting|CastToBall Other) ; проверка что это шарик???
  (bind _result (Math|Integer|DecrementInt (Variables|Default|GetLives)) ; декремент и сейв в переменную
    (:%20%20
      ;[1 1 1] инкремент + изменяем цвет шара или удаляем
      (if (> _result 0)
        (Rendering|Material|SetMaterial (Variables|Default|GetCube) 0 (Utilities|Select :Index (- (Variables|Default|GetLives) 1) :Option%200 "/Engine/MapTemplates/Materials/BasicAsset01.BasicAsset01" :Option%201 "/Engine/MapTemplates/Materials/BasicAsset03.BasicAsset03" :Option%202 "/Engine/MapTemplates/Materials/BasicAsset02.BasicAsset02")) ; меняем материал
        (else
          (Actor|DestroyActor) ; удаляем шарик
        ))
      ;[1 1 1] выводим в какой куб попали и сколько жизней осталось (лог)
      (Development|PrintString (Utilities|String|Append (Utilities|GetDisplayName (Variables|Default|GetCube)) ". Lives: " (Utilities|String|ToString(Integer) (Variables|Default|GetLives))) false true "(R=0.120634,G=1.000000,B=0.000000,A=1.000000)") ; выводим на экран айди куба в который попали
    )))

(event EventTick
  (params (DeltaSeconds :type Float%20%28single-precision%29)))

(fn ConstructionScript)