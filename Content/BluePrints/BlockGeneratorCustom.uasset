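; An actor that builds a grid of breakable Block actors at BeginPlay, apparently as a level layout for a brick-breaker style game.
; Nested loops over CountX and CountY space blocks by BlockWidth and BlockHeigth from the generator's location.
; Each block gets random Lives up to three, which selects its cube material.
; EmptySpace lowers the random minimum to zero, leaving gaps where no block spawns.
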(event EventBeginPlay
  (bind _returnvalue (Transformation|GetActorLocation))
  (bind (_x _y _z) (Math|Vector|BreakVector _returnvalue))
  ;[1 1 1] Цикл в цикле для создания кубов
  (for _index (range 0 (Variables|Default|GetcountX))
    (for _index_2 (range 0 (Variables|Default|GetcountY))
      ;[1 1 1] генерируем количество хп у кубика
      (bind _output_get (Variables|Default|SetcurrentCoubLives (Math|Random|RandomIntegerinRange (Math|Conversions|ToInteger(Boolean) (not (Variables|Default|GetemptySpace))) 3)))
      (if (> _output_get 0) ; Если > 0 то кубик создаем
        (bind _returnvalue_2 (Game|SpawnActorfromClass "/Game/BluePrints/Block.Block_C" (Math|Transform|MakeTransform (Math|Vector|MakeVector (+ (* (.X (Math|Vector|BreakVector (Math|Vector|MakeVector (Math|Conversions|ToFloat(Integer) _index) (Math|Conversions|ToFloat(Integer) _index_2) 0.0))) (Variables|Default|GetblockWidth)) _x) (+ (* (.Y (Math|Vector|BreakVector (Math|Vector|MakeVector (Math|Conversions|ToFloat(Integer) _index) (Math|Conversions|ToFloat(Integer) _index_2) 0.0))) (Variables|Default|GetblockHeigth)) _y) _z) "0, 0, 0" "1,2.000000,1") "Undefined" 0 0)) ; создает блок в заданных координатах
        ;[1 1 1] устанавливаем материал в зависимости от количества жизней
        (bind _output_get_2 (Variables|/Game/BluePrints/Block.Block_C|SetLives _returnvalue_2 (Variables|Default|GetcurrentCoubLives)))
        (Rendering|Material|SetMaterial (Variables|/Game/BluePrints/Block.Block_C|GetCube _returnvalue_2) 0 (Utilities|Select :Index (- _output_get_2 1) :Option%200 "/Engine/MapTemplates/Materials/BasicAsset01.BasicAsset01" :Option%201 "/Engine/MapTemplates/Materials/BasicAsset03.BasicAsset03" :Option%202 "/Engine/MapTemplates/Materials/BasicAsset02.BasicAsset02"))))))

(fn ConstructionScript)